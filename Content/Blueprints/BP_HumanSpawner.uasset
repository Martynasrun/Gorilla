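; BP_HumanSpawner populates the level with a crowd of humans when play begins.
; It spawns 100 BP_Human actors at random reachable navmesh points within a large radius around itself, adjusting for collisions but always spawning.
; It creates one WB_Humans widget, passes it to every human as a HUD reference, sets its human count, then adds it to the viewport.
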(event EventBeginPlay
  (bind _returnvalue (UserInterface|CreateWidget "/Game/Widgets/WB_Humans.WB_Humans_C"))
  (Variables|Default|SetHumanWidgetRef _returnvalue)
  (for _index (range 0 99)
    (Game|SpawnActorfromClass "/Game/Blueprints/BP_Human.BP_Human_C" (Math|Transform|MakeTransform (.RandomLocation (AI|Navigation|GetRandomReachablePointinRadius (Transformation|GetActorLocation) 7e+03 0 0)) "0, 0, 0" "1.000000,1.000000,1.000000") "AdjustIfPossibleButAlwaysSpawn" "MultiplyWithRoot" 0 (Variables|Default|GetHumanWidgetRef) 0)
    (Math|Integer|IncrementInt (Variables|Default|GetHumans)))
  (Variables|/Game/Widgets/WB_Humans.WB_Humans_C|SetHumans (Variables|Default|GetHumanWidgetRef) (Variables|Default|GetHumans))
  (UserInterface|Viewport|AddtoViewport (Variables|Default|GetHumanWidgetRef) 0))

(fn ConstructionScript)